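; Dummy enemy character that the player can hit or stealth-assassinate from behind.
; A sphere overlap toggles an assassinate prompt widget that faces the camera each tick.
; Damage plays a random montage, rotates the player toward the dummy via timeline, launches it along the player's forward and plays a sound.
; StealthBackAssassination disables collision, plays the victim montage, triggers delayed ragdoll and returns a reference location and rotation.
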(event `RagDoll`
  ;[1 1 1] Ragdoll
  (`|ExecutionSequence`
    (:`then_0`
      (`KismetSystemLibrary.Delay` 1.7)
      (`GameplayStatics.PlaySoundAtLocation` "/Game/Characters/Audio/Characters/Grunts-Hits/SC_Death.SC_Death" (`self.K2_GetActorLocation`) (struct) 1.0 1.0 0.0 "/Game/Characters/Audio/Characters/SA_Character.SA_Character" null null null))
    (:`then_1`
      (`KismetSystemLibrary.Delay` 2.5)
      (`PrimitiveComponent.SetSimulatePhysics` (`self.Mesh`) true))))

(event `self.Sphere.OnComponentBeginOverlap`
  (params (OverlappedComponent :type "PrimitiveComponent Object Reference") (OtherActor :type "Actor Object Reference") (OtherComp :type "PrimitiveComponent Object Reference") (OtherBodyIndex :type Integer) (bFromSweep :type Boolean) (SweepResult :type "HitResult Structure (by ref)"))
  ;[1 1 1] Assassibnate UI
  (cast `/Game/Characters/Blueprints/BP_ThirdPersonCharacter` OtherActor)
  (`SceneComponent.SetVisibility` (`self.Assassinate Widget`) true false))

(event `self.Sphere.OnComponentEndOverlap`
  (params (OverlappedComponent :type "PrimitiveComponent Object Reference") (OtherActor :type "Actor Object Reference") (OtherComp :type "PrimitiveComponent Object Reference") (OtherBodyIndex :type Integer))
  ;[1 1 1] Assassibnate UI
  (cast `/Game/Characters/Blueprints/BP_ThirdPersonCharacter` OtherActor)
  (`SceneComponent.SetVisibility` (`self.Assassinate Widget`) false false))

(event `self.ReceiveTick`
  (params (DeltaSeconds :type "Float (single-precision)"))
  ;[1 1 1] Assassibnate UI
  (`SceneComponent.K2_SetWorldRotation` (`self.Assassinate Widget`) (`KismetMathLibrary.FindLookAtRotation` (`SceneComponent.K2_GetComponentLocation` (`self.Assassinate Widget`)) (`SceneComponent.K2_GetComponentLocation` (`PlayerCameraManager.TransformComponent` (`GameplayStatics.GetPlayerCameraManager` 0)))) false false))

(event `self.ReceiveAnyDamage`
  (params (Damage :type "Float (single-precision)") (DamageType :type "DamageType Object Reference") (InstigatedBy :type "Controller Object Reference") (DamageCauser :type "Actor Object Reference"))
  ;[1 1 1] Enemy got hit
  (`self.PlayAnimMontage` (`|GetArrayItem` (`self.AnimMontages`) (`KismetMathLibrary.RandomIntegerInRange` 0 (- (`KismetArrayLibrary.Array_Length` (`self.AnimMontages`)) 1))))
  (bind _asbp_third_person_character (cast `/Game/Characters/Blueprints/BP_ThirdPersonCharacter` (`GameplayStatics.GetPlayerCharacter` 0)))
  (`self.Rotate Towards` _asbp_third_person_character)
  (`self.LaunchCharacter` (* (`KismetMathLibrary.GetForwardVector` (`self.K2_GetActorRotation` _asbp_third_person_character)) 900.0))
  (`GameplayStatics.PlaySoundAtLocation` "/Game/Characters/Audio/Characters/Grunts-Hits/SC_Death.SC_Death" (`self.K2_GetActorLocation`) (struct) 1.0 1.0 0.0 "/Game/Characters/Audio/Characters/SA_Character.SA_Character" null null null))

(event `Rotate Towards`
  (params (BP_Player :type "/Game/Characters/Blueprints/BP_ThirdPersonCharacter Object Reference"))
  (bind _capsulecomponent (`Character.CapsuleComponent` BP_Player))
  (bind (_returnvalue_roll _returnvalue_pitch _returnvalue_yaw) (`KismetMathLibrary.BreakRotator` (`SceneComponent.K2_GetComponentRotation` _capsulecomponent)))
  (bind (_returnvalue_roll_2 _returnvalue_pitch_2 _returnvalue_yaw_2) (`KismetMathLibrary.BreakRotator` (`KismetMathLibrary.FindLookAtRotation` (`SceneComponent.K2_GetComponentLocation` _capsulecomponent) (`SceneComponent.K2_GetComponentLocation` (`self.CapsuleComponent`)))))
  ;[1 1 1] Rotate player towards enemy
  (bind (_direction _value) (`Timeline|Timeline` :!via `PlayFromStart`)
    (:`Update`
      (`SceneComponent.K2_SetWorldRotation` _capsulecomponent (`KismetMathLibrary.MakeRotator` _returnvalue_roll _returnvalue_pitch (`KismetMathLibrary.Lerp` _returnvalue_yaw _returnvalue_yaw_2 _value)) false false))))

(fn `Stealth Back Assassination`
  (returns (REFLocation :type "Vector Structure") (AssassinationROtation :type "Rotator Structure"))
  (`self.SetActorEnableCollision` false)
  (`self.PlayAnimMontage` "/Game/Characters/RPG_Character/Animations/Assassination/Paired_Knife_Stealth_KidneyAndNeck_Vic_Montage.Paired_Knife_Stealth_KidneyAndNeck_Vic_Montage")
  (`self.RagDoll`)
  (`SceneComponent.SetVisibility` (`self.Assassinate Widget`) false false)
  (return (`SceneComponent.K2_GetComponentLocation` (`self.REF`)) (`self.K2_GetActorRotation`)))

(fn `UserConstructionScript`)