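; Actor component that tracks health and stamina for BP_ThirdPersonCharacter and mirrors them on its HUD.
; One tick after BeginPlay it caches the owning character, fills both stats to maximum and initializes the bars and text.
; Functions change current or maximum values, clamping increases and refreshing the HUD directly.
; Decrease functions return true on depletion, while restoring stamina also re-enables the character's CanSprint flag.
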(event `self.ReceiveBeginPlay`
  (bind _hud_wg (`/Game/Characters/Blueprints/BP_ThirdPersonCharacter.HUD_WG` (`self.PlayerCharacter_BP`)))
  (bind _hud_wg_2 (`/Game/Characters/Blueprints/BP_ThirdPersonCharacter.HUD_WG` (`self.PlayerCharacter_BP`)))
  (`KismetSystemLibrary.DelayUntilNextTick`)
  (bind _asbp_third_person_character (cast `/Game/Characters/Blueprints/BP_ThirdPersonCharacter` (`self.GetOwner`)))
  (set `self.PlayerCharacter_BP` _asbp_third_person_character)
  (bind _output_get (set `self.CurrentHealth` (`self.MaxHealth`)))
  (`ProgressBar.SetPercent` (`/Game/Characters/UI/WG_HUD.Health` _hud_wg) (/ _output_get (`self.MaxHealth`)))
  (`TextBlock.SetText` (`/Game/Characters/UI/WG_HUD.HealthText` _hud_wg) (`KismetTextLibrary.Conv_DoubleToText` (`self.CurrentHealth`) "HalfToEven"))
  (bind _output_get_2 (set `self.CurrentStamina` (`self.MaxStamina`)))
  (`ProgressBar.SetPercent` (`/Game/Characters/UI/WG_HUD.Stamina` _hud_wg_2) (/ _output_get_2 (`self.MaxStamina`)))
  (`TextBlock.SetText` (`/Game/Characters/UI/WG_HUD.StaminaText` _hud_wg_2) (`KismetTextLibrary.Conv_DoubleToText` (`self.CurrentStamina`) "HalfToEven")))

(fn `DecreaseHealth`
  (params (DamageAmount :type "Float (double-precision)"))
  (returns (IsDead :type Boolean))
  (locals (NewLocalVar :type "Float (double-precision)" :default 0.0))
  (bind _hud_wg (`/Game/Characters/Blueprints/BP_ThirdPersonCharacter.HUD_WG` (`self.PlayerCharacter_BP`)))
  (if (not (<= (`self.CurrentHealth`) 0.0))
    (bind _output_get (set `self.CurrentHealth` (- (`self.CurrentHealth`) DamageAmount)))
    (`ProgressBar.SetPercent` (`/Game/Characters/UI/WG_HUD.Health` _hud_wg) (/ _output_get (`self.MaxHealth`)))
    (`TextBlock.SetText` (`/Game/Characters/UI/WG_HUD.HealthText` _hud_wg) (`KismetTextLibrary.Conv_DoubleToText` (`self.CurrentHealth`) "HalfToEven"))
    (if (<= (`self.CurrentHealth`) 0.0)
      _
      (else
        (return false))))
  (return true))

(fn `DecreaseStamina`
  (params (DecreaseStaminaAmount :type "Float (double-precision)"))
  (returns (NoStaminaLeft :type Boolean))
  (bind _hud_wg (`/Game/Characters/Blueprints/BP_ThirdPersonCharacter.HUD_WG` (`self.PlayerCharacter_BP`)))
  (if (not (<= (`self.CurrentStamina`) 0.0))
    (bind _output_get (set `self.CurrentStamina` (- (`self.CurrentStamina`) DecreaseStaminaAmount)))
    (`ProgressBar.SetPercent` (`/Game/Characters/UI/WG_HUD.Stamina` _hud_wg) (/ _output_get (`self.MaxStamina`)))
    (`TextBlock.SetText` (`/Game/Characters/UI/WG_HUD.StaminaText` _hud_wg) (`KismetTextLibrary.Conv_DoubleToText` (`self.CurrentStamina`) "HalfToEven"))
    (if (<= (`self.CurrentStamina`) 0.0)
      _
      (else
        (return false))))
  (return true))

(fn `Increase Health`
  (params (IncreaseAmount :type "Float (double-precision)"))
  (bind _hud_wg (`/Game/Characters/Blueprints/BP_ThirdPersonCharacter.HUD_WG` (`self.PlayerCharacter_BP`)))
  (bind _output_get (set `self.CurrentHealth` (+ (`self.CurrentHealth`) IncreaseAmount)))
  (if (> _output_get (`self.MaxHealth`))
    (bind _output_get_2 (set `self.CurrentHealth` (`self.MaxHealth`))))
  (`ProgressBar.SetPercent` (`/Game/Characters/UI/WG_HUD.Health` _hud_wg) (/ _output_get_2 (`self.MaxHealth`)))
  (`TextBlock.SetText` (`/Game/Characters/UI/WG_HUD.HealthText` _hud_wg) (`KismetTextLibrary.Conv_DoubleToText` (`self.CurrentHealth`) "HalfToEven")))

(fn `Increase Max Stamina`
  (params (IncreaseMaxStaminaAmount :type "Float (double-precision)"))
  (bind _hud_wg (`/Game/Characters/Blueprints/BP_ThirdPersonCharacter.HUD_WG` (`self.PlayerCharacter_BP`)))
  (set `self.MaxStamina` (+ (`self.MaxStamina`) IncreaseMaxStaminaAmount))
  (`ProgressBar.SetPercent` (`/Game/Characters/UI/WG_HUD.Stamina` _hud_wg) (/ (`self.CurrentStamina`) (`self.MaxStamina`)))
  (`TextBlock.SetText` (`/Game/Characters/UI/WG_HUD.StaminaText` _hud_wg) (`KismetTextLibrary.Conv_DoubleToText` (`self.CurrentStamina`) "HalfToEven")))

(fn `IncreaseMaxHealth`
  (params (HealAmount :type "Float (double-precision)"))
  (bind _hud_wg (`/Game/Characters/Blueprints/BP_ThirdPersonCharacter.HUD_WG` (`self.PlayerCharacter_BP`)))
  (set `self.MaxHealth` (+ (`self.MaxHealth`) HealAmount))
  (`ProgressBar.SetPercent` (`/Game/Characters/UI/WG_HUD.Health` _hud_wg) (/ (`self.CurrentHealth`) (`self.MaxHealth`)))
  (`TextBlock.SetText` (`/Game/Characters/UI/WG_HUD.HealthText` _hud_wg) (`KismetTextLibrary.Conv_DoubleToText` (`self.CurrentHealth`) "HalfToEven")))

(fn `IncreaseStamina`
  (params (IncreaseStaminaAmount :type "Float (double-precision)"))
  (bind _hud_wg (`/Game/Characters/Blueprints/BP_ThirdPersonCharacter.HUD_WG` (`self.PlayerCharacter_BP`)))
  (set `/Game/Characters/Blueprints/BP_ThirdPersonCharacter.CanSprint` true (`self.PlayerCharacter_BP`))
  (bind _output_get (set `self.CurrentStamina` (+ (`self.CurrentStamina`) IncreaseStaminaAmount)))
  (if (> _output_get (`self.MaxStamina`))
    (bind _output_get_2 (set `self.CurrentStamina` (`self.MaxStamina`))))
  (`ProgressBar.SetPercent` (`/Game/Characters/UI/WG_HUD.Stamina` _hud_wg) (/ _output_get_2 (`self.MaxStamina`)))
  (`TextBlock.SetText` (`/Game/Characters/UI/WG_HUD.StaminaText` _hud_wg) (`KismetTextLibrary.Conv_DoubleToText` (`self.CurrentStamina`) "HalfToEven")))