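; Character component that runs a four-hit melee combo (sword swings plus a kick) and its hit detection for BP_ThirdPersonCharacter.
; Attack input plays the montage for the current AttackIndex or, mid-attack, buffers a press that SwordAttackCombo uses to chain the next hit or stop.
; A looping timer sphere-traces along the sword, while SphereTrace does a one-shot check.
; Hits on "Damagable" actors apply damage, camera shake and sound, with a cooldown on sword hits.
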(event `self.ReceiveBeginPlay`
  ;[1 1 1] Combo System
  (bind _asbp_third_person_character (cast `/Game/Characters/Blueprints/BP_ThirdPersonCharacter` (`self.GetOwner`)))
  (set `self.BP_Character` _asbp_third_person_character))

(event `Attack1`
  ;[1 1 1] Combo System
  ;;[0.2201 0.3573 0.3646] Attacks
  ;;;[1 1 1] Attack1
  (`/Engine/EditorBlueprintResources/StandardMacros.DoOnce` false :!label _label
    (:`Completed`
      (`KismetSystemLibrary.Delay` 0.2)
      (`|PlayMontage` (`Character.Mesh` (`self.BP_Character`)) "/Game/Characters/RPG_Character/Animations/SwordAttacking/Attack1_Montage.Attack1_Montage"
        (:`then`
          (set `self.AttackIndex` 1)
          (goto _label :!via `Reset`))))))

(event `EnhancedInput|/Game/ThirdPerson/Input/Actions/IA_Attack`
  (params (ActionValue :type Boolean) (ElapsedSeconds :type "Float (double-precision)") (TriggeredSeconds :type "Float (double-precision)") (InputAction :type "InputAction Object Reference" :default "/Game/ThirdPerson/Input/Actions/IA_Attack.IA_Attack"))
  ;[1 1 1] Combo System
  ;;[1 1 1] Attack Input
  (:`Started`
    (if (`self.CanAttack`)
      (`self.Sword Attack`))))

(event `Attack2`
  ;[1 1 1] Combo System
  ;;[0.2201 0.3573 0.3646] Attacks
  ;;;[1 1 1] Attack2
  (`/Engine/EditorBlueprintResources/StandardMacros.DoOnce` false :!label _label_2
    (:`Completed`
      (`KismetSystemLibrary.Delay` 0.2)
      (`|PlayMontage` (`Character.Mesh` (`self.BP_Character`)) "/Game/Characters/RPG_Character/Animations/SwordAttacking/Attack2_Montage.Attack2_Montage"
        (:`then`
          (set `self.AttackIndex` 2)
          (goto _label_2 :!via `Reset`))))))

(event `Sword Attack`
  ;[1 1 1] Combo System
  ;;[1 1 1] Sword Attack
  (if (`self.IsAttacking`)
    (set `self.SaveAttack` true)
    (else
      (set `self.IsAttacking` true)
      (switch `int` (`self.AttackIndex`) :!label _label_3
        (:`0`
          (`self.Attack1`))
        (:`1`
          (`self.Attack2`))
        (:`2`
          (`self.Attack3`))
        (:`3`
          (`self.Attack4`))))))

(event `Sword Attack Combo`
  ;[1 1 1] Combo System
  ;;[1 1 1] Sword Combo
  (if (`self.SaveAttack`)
    (set `self.SaveAttack` false)
    (goto _label_3)
    (else
      (`self.Stop Combo`))))

(event `Attack3`
  ;[1 1 1] Combo System
  ;;[0.2201 0.3573 0.3646] Attacks
  ;;;[1 1 1] Attack3
  (`/Engine/EditorBlueprintResources/StandardMacros.DoOnce` false :!label _label_4
    (:`Completed`
      (`KismetSystemLibrary.Delay` 0.2)
      (`|PlayMontage` (`Character.Mesh` (`self.BP_Character`)) "/Game/Characters/RPG_Character/Animations/SwordAttacking/Kick_Montage.Kick_Montage"
        (:`then`
          (set `self.AttackIndex` 3)
          (goto _label_4 :!via `Reset`))))))

(event `Stop Combo`
  ;[1 1 1] Combo System
  ;;[1 1 1] Stop Sword Combo / Attack
  (set `self.IsAttacking` false)
  (set `self.AttackIndex` 0))

(event `Attack4`
  ;[1 1 1] Combo System
  ;;[0.2201 0.3573 0.3646] Attacks
  ;;;[1 1 1] Attack4
  (`/Engine/EditorBlueprintResources/StandardMacros.DoOnce` false :!label _label_5
    (:`Completed`
      (`KismetSystemLibrary.Delay` 0.2)
      (`|PlayMontage` (`Character.Mesh` (`self.BP_Character`)) "/Game/Characters/RPG_Character/Animations/SwordAttacking/Attack3_Montage.Attack3_Montage"
        (:`then`
          (set `self.AttackIndex` 4)
          (goto _label_5 :!via `Reset`))))))

(event `Start Sword Trace`
  ;[1 1 1] Sword Attack
  (bind _returnvalue (`KismetSystemLibrary.K2_SetTimerDelegate` (delegate `Sword Trace Loop`) 0.001 true))
  (set `self.SwordTraceLoop` _returnvalue))

(event `Sphere Trace`
  (bind _returnvalue (`SceneComponent.K2_GetComponentLocation` (`/Game/Characters/Blueprints/BP_ThirdPersonCharacter.SphereTrace` (`self.BP_Character`))))
  ;[1 1 1] Stab & Kick
  (bind (_outhit _returnvalue_2) (`KismetSystemLibrary.SphereTraceSingle` :`Start` _returnvalue :`End` _returnvalue :`Radius` 30.0 :`TraceChannel` "TraceTypeQuery1" :`DrawDebugType` "ForDuration" :`DrawTime` 0.4))
  (if _returnvalue_2
    (bind (_bblockinghit _binitialoverlap _time _distance _location _impactpoint _normal _impactnormal _physmat _hitactor) (`GameplayStatics.BreakHitResult` _outhit))
    (if (`Actor.ActorHasTag` _hitactor "Damagable")
      (`GameplayStatics.ApplyDamage` _hitactor 10.0)
      (`GameplayStatics.PlayWorldCameraShake` "/Game/Characters/Blueprints/BP_SwordHitCamShake.BP_SwordHitCamShake_C" _location 0.0 2000.0)
      (`self.Sword HIt SFX`))))

(event `Sword Trace Loop`
  ;[1 1 1] Sword Attack
  (bind (_outhit _returnvalue) (`KismetSystemLibrary.SphereTraceSingle` :`Start` (`SceneComponent.K2_GetComponentLocation` (`/Game/Characters/Blueprints/BP_ThirdPersonCharacter.SwordTopPoint` (`self.BP_Character`))) :`End` (`SceneComponent.K2_GetComponentLocation` (`/Game/Characters/Blueprints/BP_ThirdPersonCharacter.SwordBottomPoint` (`self.BP_Character`))) :`Radius` 20.0 :`TraceChannel` "TraceTypeQuery1" :`DrawDebugType` "ForDuration" :`DrawTime` 0.4))
  (if _returnvalue
    (bind (_bblockinghit _binitialoverlap _time _distance _location _impactpoint _normal _impactnormal _physmat _hitactor) (`GameplayStatics.BreakHitResult` _outhit))
    (if (`Actor.ActorHasTag` _hitactor "Damagable")
      (`/Engine/EditorBlueprintResources/StandardMacros.DoOnce` false :!label _label_6
        (:`Completed`
          (`GameplayStatics.ApplyDamage` _hitactor 10.0)
          (`GameplayStatics.PlayWorldCameraShake` "/Game/Characters/Blueprints/BP_SwordHitCamShake.BP_SwordHitCamShake_C" _location 0.0 2000.0)
          (`self.Sword HIt SFX`)
          (`KismetSystemLibrary.Delay` 0.5)
          (goto _label_6 :!via `Reset`))))))

(event `Stop Sword Trace`
  ;[1 1 1] Sword Attack
  (`KismetSystemLibrary.K2_ClearAndInvalidateTimerHandle` (`self.SwordTraceLoop`)))

(event `Sword HIt SFX`
  ;[1 1 1] Sword Hit SFX
  (`GameplayStatics.PlaySoundAtLocation` "/Game/Characters/Audio/Characters/SwordSFX/MS_SwordHit.MS_SwordHit" (`Actor.K2_GetActorLocation` (`self.GetOwner`)) (struct) 1.0 1.0 0.0 "/Game/Characters/Audio/Characters/SA_Character.SA_Character" null null null))